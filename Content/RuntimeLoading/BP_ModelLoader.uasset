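; BP_ModelLoader loads an environment and product models at runtime from paths supplied by its JsonParserComponent.
; LoadEnvironment spawns a scaled USD stage actor from the scene path, hides the first StaticMeshActor found at BeginPlay (treated as floor) and enables collision on attached actors.
; LoadProduct loads glTF asynchronously by product ID and spawns it without built collision; the delayed collision-enable chain is unconnected.
; ProductDownloaded only logs, and T loads a test product.
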(event Custom|ProductLoaded
  (params (Asset :type Gl%20TF%20Runtime%20Asset%20Object%20Reference))
  (bind _returnvalue (Game|SpawnActorfromClass :Class "/Script/glTFRuntime.glTFRuntimeAssetActorAsync" :CollisionHandlingOverride "AdjustIfPossibleButAlwaysSpawn" :TransformScaleMethod "MultiplyWithRoot" :Asset Asset :StaticMeshConfig (Utilities|Struct|MakeglTFRuntimeStaticMeshConfig "ReadWrite" false false false 0 0 "CTF_UseDefault" false "Asset" 0 "(CacheMode=ReadWrite,UberMaterialsOverrideMap=(),MaterialsOverrideMap=(),MaterialsOverrideByNameMap=(),TexturesOverrideMap=(),ImagesOverrideMap=(),bDisableVertexColors=False,bGeneratesMipMaps=False,bMergeSectionsByMaterial=False,SpecularFactor=0.000000,bMaterialsOverrideMapInjectParams=False,ParamsMultiplier=(),ImagesConfig=(Compression=TC_Default,Group=TEXTUREGROUP_World,bSRGB=False,MaxWidth=0,MaxHeight=0,bVerticalFlip=False,bForceHDR=False,bCompressMips=False,bStreaming=False,LODBias=0,bForceAutoDetect=False,ForcePixelFormat=PF_Unknown),Variant=\"\",bSkipLoad=False,VertexColorOnlyMaterial=None,ScalarParamsOverrides=(),bLoadMipMaps=False,ForceMaterial=None,bSkipPoints=True,PointsTriangulationMode=OpenedTetrahedronWithXYInUV1ZWInUV2,PointsBaseMaterial=None,PointsScaleFactor=1.000000,bSkipLines=True,LinesTriangulationMode=OpenedTriangularPrismWithXYInUV1ZWInUV2,LinesBaseMaterial=None,LinesScaleFactor=1.000000,CustomScalarParams=(),CustomVectorParams=(),CustomTextureParams=(),bAddEpicInterchangeParams=False,MetallicRoughnessOverrideMap=(),SpecularGlossinessOverrideMap=(),ClearCoatOverrideMap=(),TransmissionOverrideMap=(),UnlitOverrideMap=(),SheenOverrideMap=())" 0 "" 0 "IfMissing" "IfMissing" false false false false 0 0 2.0 false "0.000000,0.000000,0.000000|0.000000,0.000000,-0.000000|1.000000,1.000000,1.000000") :Instigator 0)))

(event EventBeginPlay
  (bind _outactors (Actor|GetAllActorsOfClass "/Script/Engine.StaticMeshActor"))
  (Variables|Default|SetFloor (Utilities|Array|Get(acopy) _outactors)))

(event Collision|EventActorBeginOverlap
  (params (OtherActor :type Actor%20Object%20Reference)))

(event EventTick
  (params (DeltaSeconds :type Float%20%28single-precision%29)))

(event EventLoadEnvironment
  (bind _returnvalue (Game|SpawnActorfromClass "/Script/USDStage.UsdStageActor" (Math|Transform|MakeTransform "0, 0, 0" "0, 0, 0" "10.000000,10.000000,10.000000") "AlwaysSpawn" "MultiplyWithRoot" 0 0))
  (bind _returnvalue_2 (Class|JsonParserComponent|GetSceneDataPath (Variables|Default|GetJsonParserComponent)))
  (Class|UsdStageActor|SetRootLayer _returnvalue _returnvalue_2)
  (Rendering|SetVisibility (Variables|/Script/Engine.StaticMeshActor|GetStaticMeshComponent (Variables|Default|GetFloor)) false false)
  (Class|ModelLoader|EnableActorsCollision (Actor|GetAttachedActors _returnvalue true true)))

(event EventProductDownloaded
  (params (ProductID :type String))
  (Utilities|String|LogString (Utilities|String|Append ProductID " loaded")))

(event EventLoadProduct
  (params (ProductID :type String))
  (bind _returnvalue (Class|JsonParserComponent|GetProductDataCollection (Variables|Default|GetJsonParserComponent)))
  (Class|GlTFRuntimeFunctionLibrary|GlTFLoadAssetfromFilenameAsync :Filename (.modelpath (.Value (Utilities|Map|Find _returnvalue ProductID))) :Completed (delegate Custom|ProductLoaded)))

(event Input|KeyboardEvents|DebugKeyT
  (params (Key :type Key%20Structure :default "None") (ActionValue :type Input%20Action%20Value%20Structure))
  (:Pressed
    (Class|ModelLoader|LoadProduct "pid2")))

(fn ConstructionScript)