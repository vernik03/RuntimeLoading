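; Player controller that spawns a BP_ModelLoader and turns Enhanced Input actions into placement controls for runtime-loaded models.
; One axis input either rotates or scales the loader's Anchor via a toggle, with scaling additive above 1 and multiplicative otherwise.
; Place releases the placeholder item and resets its transform offsets, or selects the anchor's temporary actor.
; Mouse and camera inputs switch between cursor and look modes, with camera input also updating the anchor's StopMoving flag.
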(event Input|EnhancedActionEvents|EnhancedInputActionIA_RotateCamera
  (params (ActionValue :type Boolean) (ElapsedSeconds :type Float%20%28double-precision%29) (TriggeredSeconds :type Float%20%28double-precision%29) (InputAction :type Input%20Action%20Object%20Reference :default "/Game/RuntimeLoading/Game/Input/IA_RotateCamera.IA_RotateCamera"))
  (bind _self self)
  (:Started
    (if (Variables|Default|GetbShowMouseCursor)
      (Variables|/Game/RuntimeLoading/BP_MouseAnchor.BP_MouseAnchor_C|SetbStopMoving (Variables|/Game/RuntimeLoading/BP_ModelLoader.BP_ModelLoader_C|GetAnchor (Variables|Default|GetModelLoader)) (Variables|Default|GetbShowMouseCursor) :!label _label)
      (bind _output_get (Variables|Default|SetbShowMouseCursor (not (Variables|Default|GetbShowMouseCursor))))
      (Input|SetIgnoreLookInput _output_get)
      (if _output_get
        (Input|SetInputModeGameandUI _self 0 "DoNotLock" true false)
        (else
          (Input|SetInputModeGameOnly _self false)))))
  (:Completed
    (if (not (Variables|Default|GetbShowMouseCursor))
      (if (Variables|Default|GetbMouseEnabled)
        (goto _label)))))

(event Input|EnhancedActionEvents|EnhancedInputActionIA_Rotate_Scale_Change
  (params (ActionValue :type Boolean) (ElapsedSeconds :type Float%20%28double-precision%29) (TriggeredSeconds :type Float%20%28double-precision%29) (InputAction :type Input%20Action%20Object%20Reference :default "/Game/RuntimeLoading/Game/Input/IA_Rotate_Scale_Change.IA_Rotate_Scale_Change"))
  (:Started
    (Variables|Default|SetbRotating (not (Variables|Default|GetbRotating)))))

(event Input|EnhancedActionEvents|EnhancedInputActionIA_Rotate_Scale
  (params (ActionValue :type Float%20%28double-precision%29) (ElapsedSeconds :type Float%20%28double-precision%29) (TriggeredSeconds :type Float%20%28double-precision%29) (InputAction :type Input%20Action%20Object%20Reference :default "/Game/RuntimeLoading/Game/Input/IA_Rotate_Scale.IA_Rotate_Scale"))
  (bind _returnvalue (Math|Float|Absolute(Float) ActionValue))
  (bind _modelloader (Variables|Default|GetModelLoader))
  (bind _returnvalue_2 (* _returnvalue 2.0))
  (bind _anchor (Variables|/Game/RuntimeLoading/BP_ModelLoader.BP_ModelLoader_C|GetAnchor _modelloader))
  ;[0.15 0.15 0.15 0.5] Scale and Rotate
  (if (Variables|Default|GetbRotating)
    (Variables|/Game/RuntimeLoading/BP_MouseAnchor.BP_MouseAnchor_C|SetAdditionalRotation _anchor (+ (Variables|/Game/RuntimeLoading/BP_MouseAnchor.BP_MouseAnchor_C|GetAdditionalRotation _anchor) ActionValue))
    (elif (> (Variables|/Game/RuntimeLoading/BP_MouseAnchor.BP_MouseAnchor_C|GetAdditionalScale _anchor) 1.0)
      (Variables|/Game/RuntimeLoading/BP_MouseAnchor.BP_MouseAnchor_C|SetAdditionalScale _anchor (+ ActionValue (Variables|/Game/RuntimeLoading/BP_MouseAnchor.BP_MouseAnchor_C|GetAdditionalScale _anchor)))
      (elif (< ActionValue 0.0)
        (Variables|/Game/RuntimeLoading/BP_MouseAnchor.BP_MouseAnchor_C|SetAdditionalScale _anchor (/ (Variables|/Game/RuntimeLoading/BP_MouseAnchor.BP_MouseAnchor_C|GetAdditionalScale _anchor) _returnvalue_2))
        (else
          (Variables|/Game/RuntimeLoading/BP_MouseAnchor.BP_MouseAnchor_C|SetAdditionalScale _anchor (* (Variables|/Game/RuntimeLoading/BP_MouseAnchor.BP_MouseAnchor_C|GetAdditionalScale _anchor) _returnvalue_2)))))))

(event Input|EnhancedActionEvents|EnhancedInputActionIA_Place
  (params (ActionValue :type Boolean) (ElapsedSeconds :type Float%20%28double-precision%29) (TriggeredSeconds :type Float%20%28double-precision%29) (InputAction :type Input%20Action%20Object%20Reference :default "/Game/RuntimeLoading/Game/Input/IA_Place.IA_Place"))
  (bind _modelloader (Variables|Default|GetModelLoader))
  (bind _anchor (Variables|/Game/RuntimeLoading/BP_ModelLoader.BP_ModelLoader_C|GetAnchor _modelloader))
  (:Started
    (Utilities|IsValid (Variables|/Game/RuntimeLoading/BP_MouseAnchor.BP_MouseAnchor_C|GetPlaceholderItem _anchor)
      (:Is%20Valid
        (Variables|/Game/RuntimeLoading/BP_MouseAnchor.BP_MouseAnchor_C|SetPlaceholderItem _anchor 0)
        (Variables|/Game/RuntimeLoading/BP_MouseAnchor.BP_MouseAnchor_C|SetAdditionalRotation _anchor 0.0)
        (Variables|/Game/RuntimeLoading/BP_MouseAnchor.BP_MouseAnchor_C|SetAdditionalScale _anchor 1.0))
      (:Is%20Not%20Valid
        (Utilities|IsValid (Variables|/Game/RuntimeLoading/BP_MouseAnchor.BP_MouseAnchor_C|GetTempActor _anchor)
          (:Is%20Valid
            (Default|SelectActor _anchor)))))))

(event Input|EnhancedActionEvents|EnhancedInputActionIA_EnableMouse
  (params (ActionValue :type Boolean) (ElapsedSeconds :type Float%20%28double-precision%29) (TriggeredSeconds :type Float%20%28double-precision%29) (InputAction :type Input%20Action%20Object%20Reference :default "/Game/RuntimeLoading/Game/Input/IA_EnableMouse.IA_EnableMouse"))
  (bind _self self)
  (:Started
    (Variables|Default|SetbMouseEnabled (not (Variables|Default|GetbShowMouseCursor)))
    (bind _output_get (Variables|Default|SetbShowMouseCursor (not (Variables|Default|GetbShowMouseCursor))))
    (Input|SetIgnoreLookInput _output_get)
    (if _output_get
      (Input|SetInputModeGameandUI _self 0 "DoNotLock" true false)
      (else
        (Input|SetInputModeGameOnly _self false)))))

(event EventBeginPlay
  (bind _returnvalue (Game|SpawnActorfromClass "/Game/RuntimeLoading/BP_ModelLoader.BP_ModelLoader_C" (Math|Transform|MakeTransform "0, 0, 0" "0, 0, 0" "1.000000,1.000000,1.000000") "Undefined" "MultiplyWithRoot" 0 0))
  (Variables|Default|SetModelLoader _returnvalue))

(event EventTick
  (params (DeltaSeconds :type Float%20%28single-precision%29)))

(fn ConstructionScript)